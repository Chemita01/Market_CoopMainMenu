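; Main menu GameState for the cooperative mode that finalizes the local player roster and launches the game level.
; StartGame loops over PlayerArray, removing local players whose controller has no valid PlayerSlot and registering those found in the Game Instance's PlayersReady map through AddPlayer.
; It then opens L_Overview, using a cached getter for the GI_Cooperative reference throughout.
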(event `StartGame`
  (for (_array_element _array_index) (`self.PlayerArray`)
    (bind _aspc_main_menu (cast `/Game/Cooperative/Core/MainMenu/BP_PlayerController_MainMenu` (`PlayerState.GetPlayerController` _array_element))) ; Se hace un cast al Player Controller para recoger el Player Slot
    (bind _player_slot (`/Game/Cooperative/Core/MainMenu/BP_PlayerController_MainMenu.Player Slot` _aspc_main_menu))
    (if (<= _player_slot -1)
      (`GameplayStatics.RemovePlayer` _aspc_main_menu true) ; Eliminar jugador local
      (else
        (bind _s_playerstruct_index (break `/Game/Cooperative/Structs/S_PlayerStruct` (make `/Game/Cooperative/Structs/S_PlayerStruct` _player_slot _array_index "None")))
        (if (`.ReturnValue` (`BlueprintMapLibrary.Map_Find` (`/Game/Cooperative/Core/GI_Cooperative.Players Ready` (`self.getGIRef`)) _s_playerstruct_index))
          (`/Game/Cooperative/Core/GI_Cooperative.AddPlayer` (`self.getGIRef`) (make `/Game/Cooperative/Structs/S_PlayerStruct` _player_slot _array_index "None")) ; Añadir jugador al array de jugadores con la información necesaria
        ))))
  (`GameplayStatics.OpenLevelBySoftObjectPtr` "/Game/Cooperative/Levels/L_Overview.L_Overview") ; Abrir nivel de juego una vez el bucle haya finalizado
)

(fn `getGIRef`
  (returns (`As GI Cooperative` :type "/Game/Cooperative/Core/GI_Cooperative Object Reference"))
  ;[0.02083 0.02083 0.02083 0.036] Función para referenciar el Game Instance
  (`self.As GI Coop`
    (:`then`
      _)
    (:`else`
      (bind _asgi_cooperative (cast `/Game/Cooperative/Core/GI_Cooperative` (`GameplayStatics.GetGameInstance`)))
      (set `self.As GI Coop` _asgi_cooperative)))
  (return (`self.As GI Coop`)))

(fn `UserConstructionScript`)