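; HUD for the cooperative main menu, where players join and ready up.
; On BeginPlay it creates and displays WBP_MainMenu, only for the owning player controller with ID 0.
; Its functions forward join, leave, ready and unready calls to that widget so player controllers can invoke them, passing back the widget's results where provided.
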(event `self.ReceiveBeginPlay`
  ;[0.02083 0.02083 0.02083 0.036] Evento "BeginPlay" para crear el widget del menú principal donde los jugadores se unirán
  (if (== (`GameplayStatics.GetPlayerControllerID` (`self.GetOwningPlayerController`)) 0)
    (bind _returnvalue (`|CreateWidget` "/Game/Cooperative/UI/WBP_MainMenu.WBP_MainMenu_C"))
    (bind _output_get (set `self.W Main Menu` _returnvalue))
    (`UserWidget.AddToViewport` _output_get 0)))

(fn `AddPlayerReady`
  (returns (PlayersReady :type "Map of Integer to Boolean"))
  ;[0.02083 0.02083 0.02083 0.036] Función que llama al "Player Ready" del menú principal para poder ser ejecutado desde el Player Controller
  (bind _w_main_menu (`self.W Main Menu`)
    (:`then`
      (bind _playersready (`/Game/Cooperative/UI/WBP_MainMenu.AddPlayerReady` _w_main_menu))
      (return _playersready))
    (:`else`)))

(fn `AddPlayerToSlot`
  (returns (NewPlayerSlot :type Integer))
  ;[0.02083 0.02083 0.02083 0.036] Función que llama al "Player Join" del menú principal para poder ser ejecutado desde el Player Controller
  (bind _w_main_menu (`self.W Main Menu`)
    (:`then`
      (bind _playerslot (`/Game/Cooperative/UI/WBP_MainMenu.AddPlayerJoin` _w_main_menu))
      (return _playerslot))
    (:`else`
      (return 0))))

(fn `Remove Player From Ready'sPlayer`
  (params (`Player Slot` :type Integer))
  (returns (`Player Slot from remove` :type Integer))
  ;[0.02083 0.02083 0.02083 0.036] Función que llama al "Remove Player Ready" del menú principal para poder ser ejecutado desde el Player Controller
  (bind _w_main_menu (`self.W Main Menu`)
    (:`then`
      (bind _player_slot_from_remove (`/Game/Cooperative/UI/WBP_MainMenu.RemovePlayerReady` _w_main_menu `Player Slot`))
      (return _player_slot_from_remove))
    (:`else`)))

(fn `Remove Player From Slot`
  (params (`Player Slot` :type Integer))
  ;[0.02083 0.02083 0.02083 0.036] Función que llama al "Remove Player Join" del menú principal para poder ser ejecutado desde el Player Controller
  (bind _w_main_menu (`self.W Main Menu`)
    (:`then`
      (`/Game/Cooperative/UI/WBP_MainMenu.RemovePlayerJoin` _w_main_menu `Player Slot`))
    (:`else`)))

(fn `UserConstructionScript`)